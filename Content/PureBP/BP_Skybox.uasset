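; BP_Skybox is a skybox actor that switches the scene between day and night looks.
; Its Day and Night events each swap the static mesh's sky material and set the intensity of the referenced LightAll light, dimming it at night.
; The switch is instant, with no tick or blending, and Day also prints the light's display name.
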(event Custom|Day
  (bind _lightall (Variables|Default|GetlightAll))
  ;[1 1 1] Day Night
  (Rendering|Material|SetMaterial (Variables|Default|GetStaticMesh) 0 "/Engine/MapTemplates/MASTER_Sky_Material.MASTER_Sky_Material")
  (Rendering|Components|Light|SetIntensity (Variables|/Script/Engine.Light|GetLightComponent _lightall) 1.8)
  (Development|PrintString (Utilities|GetDisplayName _lightall)))

(event Custom|Night
  ;[1 1 1] Day Night
  (Rendering|Material|SetMaterial (Variables|Default|GetStaticMesh) 0 "/Engine/MapTemplates/Sky/M_Procedural_Sky_Night.M_Procedural_Sky_Night")
  (Rendering|Components|Light|SetIntensity (Variables|/Script/Engine.Light|GetLightComponent (Variables|Default|GetlightAll)) 0.09))

(event EventBeginPlay)

(event Collision|EventActorBeginOverlap
  (params (OtherActor :type Actor%20Object%20Reference)))

(event EventTick
  (params (DeltaSeconds :type Float%20%28single-precision%29)))

(fn ConstructionScript)