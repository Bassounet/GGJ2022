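; Scarecrow enemy that threatens the first-person player with sudden, sound-cued jumps toward them.
; Entering its sphere stores the player's position, flags them as menaced and shakes their camera; leaving clears the threat.
; While they remain inside, a looping timer sweeps the enemy to that stored entry position.
; After first contact it always faces the player; Jour/Nuit events swap its material, and the footstep timer is unconnected.
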(event OnComponentBeginOverlap(Sphere)
  (params (OverlappedComponent :type Primitive%20Component%20Object%20Reference) (OtherActor :type Actor%20Object%20Reference) (OtherComp :type Primitive%20Component%20Object%20Reference) (OtherBodyIndex :type Integer) (bFromSweep :type Boolean) (SweepResult :type Hit%20Result%20Structure%20%28by%20ref%29))
  (bind _asfirst_person_character (Utilities|Casting|CastToFirstPersonCharacter OtherActor))
  (Variables|Default|SetplyerAldyViewed true)
  (Variables|Default|SetPlayerViewed true)
  (Variables|Default|SetLocationPlayer (Math|Conversions|ToTransform(Vector) (Transformation|GetActorLocation _asfirst_person_character)))
  (Variables|/Game/FirstPersonBP/Blueprints/FirstPersonCharacter.FirstPersonCharacter_C|SetInMenace _asfirst_person_character true)
  (Default|CamShake _asfirst_person_character))

(event OnComponentEndOverlap(Sphere)
  (params (OverlappedComponent :type Primitive%20Component%20Object%20Reference) (OtherActor :type Actor%20Object%20Reference) (OtherComp :type Primitive%20Component%20Object%20Reference) (OtherBodyIndex :type Integer))
  (bind _asfirst_person_character (Utilities|Casting|CastToFirstPersonCharacter OtherActor))
  (Variables|Default|SetPlayerViewed false)
  (Variables|Default|SetLocationPlayer (Math|Conversions|ToTransform(Vector) (Transformation|GetActorLocation _asfirst_person_character)))
  (Variables|/Game/FirstPersonBP/Blueprints/FirstPersonCharacter.FirstPersonCharacter_C|SetInMenace _asfirst_person_character false))

(event Custom|Nuit
  ;[1 1 1] Jour/ Nuit
  (Rendering|Material|SetMaterial (Variables|Default|GetStaticMesh) 0 "/Game/3D/Epouvantail/Textures/M_Epouvantaiiil_corps.M_Epouvantaiiil_corps"))

(event Custom|Jour
  ;[1 1 1] Jour/ Nuit
  (Rendering|Material|SetMaterial (Variables|Default|GetStaticMesh) 0 "/Game/FirstPerson/Meshes/FirstPersonProjectileMaterial.FirstPersonProjectileMaterial"))

(event Custom|TryTP
  (if (Variables|Default|GetPlayerViewed)
    (Audio|PlaySoundatLocation "/Game/SND/monstre.monstre" (Transformation|GetActorLocation) "0, 0, 0" 1.0 1.0 0.0 "/Game/SND/Faya.Faya" 0 0)
    (Transformation|SetActorLocationAndRotation (Math|Transform|TransformLocation (Variables|Default|GetLocationPlayer) "0, 0, 0") "0, 0, 0" true)))

(event Custom|Play
  (Audio|PlaySoundatLocation "/Game/SND/Walking/Walking.Walking" (Transformation|GetActorLocation) "0, 0, 0" 1.0 1.0 0.0 0 0 0))

(event EventTick
  (params (DeltaSeconds :type Float%20%28single-precision%29))
  ;[1 1 1] Look At Me Now
  (if (Variables|Default|GetplyerAldyViewed)
    (Transformation|SetActorRotation (Math|Rotator|FindLookatRotation (Transformation|GetActorLocation) (Transformation|GetActorLocation (stale OnComponentBeginOverlap(Sphere) _asfirst_person_character))))))

(event EventBeginPlay
  (Utilities|Time|SetTimerbyEvent (delegate Custom|TryTP) 5.0 true)
  (if (Variables|Default|GetPlayerViewed)
    (Audio|PlaySoundatLocation "/Game/SND/monstre.monstre" (Transformation|GetActorLocation) "0, 0, 0" 1.0 1.0 0.0 "/Game/SND/Faya.Faya" 0 0)
    (Transformation|SetActorLocationAndRotation (Math|Transform|TransformLocation (Variables|Default|GetLocationPlayer) "0, 0, 0") "0, 0, 0" true)))

(fn ConstructionScript)