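; BP_BRUIT is a noise hazard actor that raises the player's paranoia and slows them on contact, with its mesh set at BeginPlay.
; Any Box overlap plays a 2D sound; if the AdyTouched guard is clear, FirstPersonCharacter gets Ouch, added paranoia and Ralenti.
; When the character leaves, a short delay clears the guard, then ReturnSPeed is called after TimeToSlow.
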(event OnComponentBeginOverlap(Box)
  (params (OverlappedComponent :type Primitive%20Component%20Object%20Reference) (OtherActor :type Actor%20Object%20Reference) (OtherComp :type Primitive%20Component%20Object%20Reference) (OtherBodyIndex :type Integer) (bFromSweep :type Boolean) (SweepResult :type Hit%20Result%20Structure%20%28by%20ref%29))
  ;[1 1 1] Ouch
  (Audio|PlaySound2D (Variables|Default|GetSoundToPlay) 1.0 1.0 0.0 0 0)
  (if (not (Variables|Default|GetAdyTouched))
    (bind _asfirst_person_character (Utilities|Casting|CastToFirstPersonCharacter OtherActor))
    (Default|Ouch _asfirst_person_character)
    (Variables|/Game/FirstPersonBP/Blueprints/FirstPersonCharacter.FirstPersonCharacter_C|SetCurrentParanoiaPT _asfirst_person_character (+ (Variables|/Game/FirstPersonBP/Blueprints/FirstPersonCharacter.FirstPersonCharacter_C|GetCurrentParanoiaPT _asfirst_person_character) (Variables|Default|GetParanoiaToAdd)))
    (Variables|Default|SetAdyTouched true)
    (Default|Ralenti _asfirst_person_character)))

(event OnComponentEndOverlap(Box)
  (params (OverlappedComponent :type Primitive%20Component%20Object%20Reference) (OtherActor :type Actor%20Object%20Reference) (OtherComp :type Primitive%20Component%20Object%20Reference) (OtherBodyIndex :type Integer))
  ;[1 1 1] Ouch
  (bind _asfirst_person_character (Utilities|Casting|CastToFirstPersonCharacter OtherActor))
  (Utilities|FlowControl|Delay 0.2)
  (Variables|Default|SetAdyTouched false)
  (Utilities|FlowControl|Delay (Variables|Default|GetTimeToSlow))
  (Default|ReturnSPeed _asfirst_person_character))

(event Collision|EventActorBeginOverlap
  (params (OtherActor :type Actor%20Object%20Reference)))

(event EventTick
  (params (DeltaSeconds :type Float%20%28single-precision%29)))

(event EventBeginPlay
  ;[1 1 1] ChangeMesh
  (Components|StaticMesh|SetStaticMesh (Variables|Default|GetStaticMesh) (Variables|Default|GetNew%20Mesh)))

(fn ConstructionScript)